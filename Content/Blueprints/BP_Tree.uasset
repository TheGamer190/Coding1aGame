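; BP_Tree is a tree actor that grows in random steps after BeginPlay.
; While GrowthCount is above zero, it waits a random few seconds, enlarges the Model's scale by a random amount and decrements the count.
; When the count runs out, it enables query and physics collision on the Model and makes the Sphere component visible.
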(event `self.ReceiveBeginPlay`
  (bind _model (`self.Model`))
  (if (> (`self.growthCount`) 0) :!label _label
    (`KismetSystemLibrary.Delay` (`KismetMathLibrary.RandomFloatInRange` 3.0 8.0))
    (`SceneComponent.SetRelativeScale3D` _model (+ (`SceneComponent.K2_GetComponentScale` _model) (`KismetMathLibrary.RandomFloatInRange` 0.05 0.3)))
    (`/Engine/EditorBlueprintResources/StandardMacros.DecrementInt` (`self.growthCount`)
      (:`  `
        (goto _label)))
    (else
      (`PrimitiveComponent.SetCollisionEnabled` (`self.Model`) "QueryAndPhysics")
      (`SceneComponent.SetVisibility` (`self.Sphere`) true false))))

(fn `UserConstructionScript`)