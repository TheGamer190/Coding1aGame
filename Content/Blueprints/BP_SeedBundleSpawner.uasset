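; Spawner actor that scatters BP_SeedBundle actors at random positions over a fixed rectangular area at a constant low height.
; On BeginPlay, a looped-back branch spawns bundles and decrements Counter until it reaches zero.
; The SpawnBundles event enters past the check, so it always spawns at least one bundle before rejoining the loop.
; Each spawn overwrites NewVar with a single-element array.
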(event `self.ReceiveBeginPlay`
  (if (> (`self.Counter`) 0) :!label _label
    (bind _returnvalue (`|SpawnActorFromClass` "/Game/Blueprints/BP_SeedBundle.BP_SeedBundle_C" (`KismetMathLibrary.MakeTransform` (`KismetMathLibrary.MakeVector` (`KismetMathLibrary.RandomFloatInRange` -6230.0 6230.0) (`KismetMathLibrary.RandomFloatInRange` -6000.0 6000.0) 1.0)) "Undefined" "MultiplyWithRoot" null null :!label _label_2))
    (set `self.NewVar` (`|MakeArray` _returnvalue))
    (`/Engine/EditorBlueprintResources/StandardMacros.DecrementInt` (`self.Counter`)
      (:`  `
        (goto _label)))))

(event `SpawnBundles`
  (goto _label_2))

(fn `UserConstructionScript`)