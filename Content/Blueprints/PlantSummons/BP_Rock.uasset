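; BP_Rock is a summoned rock plant that grows, then shoots rock bullets at enemies.
; On BeginPlay it scales up in randomly timed steps, then enables collision and despawns 30 seconds later.
; Overlapping a BP_Enemy stores it as target and, once grown, starts a delayed loop spawning BP_RockBullet aimed at it and launched by force.
; The loop repeats until an enemy ends overlap.
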(event `DespawnPlant`
  (`KismetSystemLibrary.Delay` 30.0)
  (`self.K2_DestroyActor`))

(event `self.ReceiveBeginPlay`
  (bind _rockbase (`self.RockBase`))
  (if (> (`self.growthCount`) 0) :!label _label
    (`KismetSystemLibrary.Delay` (`KismetMathLibrary.RandomFloatInRange` 3.0 8.0))
    (`SceneComponent.SetRelativeScale3D` _rockbase (+ (`SceneComponent.K2_GetComponentScale` _rockbase) (`KismetMathLibrary.RandomFloatInRange` 0.01 0.03)))
    (`/Engine/EditorBlueprintResources/StandardMacros.DecrementInt` (`self.growthCount`)
      (:`  `
        (goto _label)))
    (else
      (`PrimitiveComponent.SetCollisionEnabled` (`self.RockBase`) "QueryAndPhysics")
      (`PrimitiveComponent.SetCollisionEnabled` (`self.RockShooter`) "QueryAndPhysics")
      (set `self.isEnabled` true)
      (`self.DespawnPlant`))))

(event `ShootRock`
  (bind _returnvalue_location (`KismetMathLibrary.BreakTransform` (`SceneComponent.K2_GetComponentToWorld` (`self.Spawn point`))))
  (if (`self.isEnabled`)
    (`KismetSystemLibrary.Delay` 0.2 :!label _label_2)
    (bind _returnvalue (`|SpawnActorFromClass` "/Game/Blueprints/PlantSummons/BP_RockBullet.BP_RockBullet_C" (`KismetMathLibrary.MakeTransform` _returnvalue_location (`KismetMathLibrary.MakeRotationFromAxes` (`KismetMathLibrary.Normal` (- (`SceneComponent.K2_GetComponentLocation` (`Actor.RootComponent` (`self.enemy`))) (`SceneComponent.K2_GetComponentLocation` (`self.Spawn point`)))))) "Undefined" "MultiplyWithRoot" null null))
    (bind _rock (`/Game/Blueprints/PlantSummons/BP_RockBullet.Rock` _returnvalue))
    (`PrimitiveComponent.AddForce` _rock (* (`SceneComponent.GetForwardVector` _rock) (`self.shootForce`)) "None" true)
    (if (== (`self.isEnemyInRange`) true)
      (goto _label_2))))

(event `self.ReceiveActorBeginOverlap`
  (params (OtherActor :type "Actor Object Reference"))
  (bind _asbp_enemy (cast `/Game/Blueprints/BP_Enemy` OtherActor))
  (set `self.enemy` _asbp_enemy)
  (set `self.isEnemyInRange` true)
  (if (== (`self.isEnemyInRange`) true)
    (`self.ShootRock`)))

(event `self.ReceiveActorEndOverlap`
  (params (OtherActor :type "Actor Object Reference"))
  (cast `/Game/Blueprints/BP_Enemy` OtherActor)
  (set `self.isEnemyInRange` false))

(fn `UserConstructionScript`)