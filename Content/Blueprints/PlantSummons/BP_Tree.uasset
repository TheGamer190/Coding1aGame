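; BP_Tree is a summoned plant that grows in place and then slows enemies that overlap it.
; BeginPlay loops through randomly delayed scale increments until GrowthCount runs out, then enables model collision, shows the Sphere and sets IsEnabled.
; Once enabled, beginning an overlap halves a BP_Enemy's MoveSpeed, which resets to normal after a short delay or when the overlap ends.
; The fully grown tree destroys itself after a fixed lifetime.
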(event `DespawnPlant`
  ; Despawn actor after 90 sec
  (`KismetSystemLibrary.Delay` 90.0)
  (`self.K2_DestroyActor`))

(event `self.ReceiveActorEndOverlap`
  (params (OtherActor :type "Actor Object Reference"))
  ; Return enemy speed
  (bind _asbp_enemy (cast `/Game/Blueprints/BP_Enemy` OtherActor))
  (set `/Game/Blueprints/BP_Enemy.moveSpeed` 1.0 _asbp_enemy))

(event `self.ReceiveActorBeginOverlap`
  (params (OtherActor :type "Actor Object Reference"))
  ; Slow enemy down
  (if (`self.isEnabled`)
    (bind _asbp_enemy (cast `/Game/Blueprints/BP_Enemy` OtherActor))
    (set `/Game/Blueprints/BP_Enemy.moveSpeed` 0.5 _asbp_enemy)
    (`KismetSystemLibrary.Delay` 5.0)
    (set `/Game/Blueprints/BP_Enemy.moveSpeed` 1.0 _asbp_enemy)))

(event `self.ReceiveBeginPlay`
  (bind _model (`self.Model`))
  ; Grow tree
  (if (> (`self.growthCount`) 0) :!label _label
    (`KismetSystemLibrary.Delay` (`KismetMathLibrary.RandomFloatInRange` 1.0 3.0))
    (`SceneComponent.SetRelativeScale3D` _model (+ (`SceneComponent.K2_GetComponentScale` _model) (`KismetMathLibrary.RandomFloatInRange` 0.05 0.3)))
    (`/Engine/EditorBlueprintResources/StandardMacros.DecrementInt` (`self.growthCount`)
      (:`  `
        (goto _label)))
    (else
      (`PrimitiveComponent.SetCollisionEnabled` (`self.Model`) "QueryAndPhysics")
      (`SceneComponent.SetVisibility` (`self.Sphere`) true false)
      (set `self.isEnabled` true)
      (`self.DespawnPlant`))))

(fn `UserConstructionScript`)