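; BP_DialogueManager shows a timed sequence of dialogue lines on the player's UI.
; DisplayNextLine steps through the DialogueStrings array, showing each entry for three seconds through a self-looping Delay, then clears the text and resets the index.
; ShowDialogue and HideDialogue write to the Dialogue text in the UI of player 0's BP_ThirdPersonCharacter.
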(event `DisplayNextLine`
  (if (!= (`self.arrayIndex`) (`KismetArrayLibrary.Array_Length` (`self.dialogueStrings`))) :!label _label
    (`self.ShowDialogue`)
    (`/Engine/EditorBlueprintResources/StandardMacros.IncrementInt` (`self.arrayIndex`)
      (:`  `
        (`KismetSystemLibrary.Delay` 3.0)
        (goto _label)))
    (else
      (`self.HideDialogue`))))

(event `ShowDialogue`
  (bind _asbp_third_person_character (cast `/Game/ThirdPerson/Blueprints/BP_ThirdPersonCharacter` (`GameplayStatics.GetPlayerCharacter` 0)))
  (`TextBlock.SetText` (`/Game/UI/UI_PlayerUI.Dialogue` (`/Game/ThirdPerson/Blueprints/BP_ThirdPersonCharacter.UI` _asbp_third_person_character)) (`|GetArrayItem` (`self.dialogueStrings`) (`self.arrayIndex`))))

(event `HideDialogue`
  (bind _asbp_third_person_character (cast `/Game/ThirdPerson/Blueprints/BP_ThirdPersonCharacter` (`GameplayStatics.GetPlayerCharacter` 0)))
  (`TextBlock.SetText` (`/Game/UI/UI_PlayerUI.Dialogue` (`/Game/ThirdPerson/Blueprints/BP_ThirdPersonCharacter.UI` _asbp_third_person_character)) "")
  (set `self.arrayIndex` 0))

(fn `UserConstructionScript`)